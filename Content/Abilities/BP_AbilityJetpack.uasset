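; Jetpack ability that pushes the owning character upward for a limited airtime budget.
; Activation with time remaining switches movement to Falling and starts a timer, which deactivation invalidates.
; Each update drains the remaining time and applies vertical force from a helper function, stopping the Jump-tagged ability when time runs out.
; A movement-mode delegate refills the budget and broadcasts the reset when the owner returns to Walking.
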(event `self.InitializeAbility`
  (params (Owner :type "MRCharacter Object Reference"))
  (`parent.InitializeAbility` Owner)
  (set `self.TimeLeft` (`self.JetpackTime`))
  (add `Character.MovementModeChangedDelegate` Owner (delegate `MovementModeChangedDelegate_Event_0`)))

(event `MovementModeChangedDelegate_Event_0`
  (params (Character :type "Character Object Reference") (PrevMovementMode :type "EMovementMode Enum" :default "MOVE_None") (PreviousCustomMode :type Byte))
  ;[1 1 1] Recharge Jetpack when landed
  (if (`|EnumEquality` (`CharacterMovementComponent.MovementMode` (`Character.CharacterMovement` Character)) "MOVE_Walking")
    (bind _output_get (set `self.TimeLeft` (`self.JetpackTime`)))
    (`self.OnTimeLeftReset` _output_get)))

(event `self.ActivateAbility`
  ;[1 1 1] Activate the ability
  (`parent.ActivateAbility`)
  (`self.OwnerCharacter`
    (:`then`
      (if (> (`self.TimeLeft`) 0.0)
        (bind _returnvalue (`KismetSystemLibrary.K2_SetTimerDelegate` (`|CreateDelegate` :!event `StopAbility`) (`self.TimeLeft`)))
        (set `self.JetpackHandle` _returnvalue)
        (`CharacterMovementComponent.SetMovementMode` (`Character.CharacterMovement` (`self.OwnerCharacter`)) "MOVE_Falling" 0)))
    (:`else`)))

(event `self.DeactivateAbility`
  ;[1 1 1] Deactivate the ability
  (`parent.DeactivateAbility`)
  (`KismetSystemLibrary.K2_InvalidateTimerHandle` (`self.JetpackHandle`)))

(event `self.UpdateAbility`
  (params (DeltaTime :type "Float (single-precision)"))
  ;[1 1 1] Ability Update
  (bind _output_get (set `self.TimeLeft` (- (`self.TimeLeft`) DeltaTime)))
  (if (> _output_get 0.0)
    (`CharacterMovementComponent.AddForce` (`Character.CharacterMovement` (`self.OwnerCharacter`)) (`KismetMathLibrary.MakeVector` 0.0 0.0 (* (+ (/ (* (`self.MaxHeight`) 2.0) (`self.JetpackTime`)) (`KismetMathLibrary.Abs` (`MovementComponent.GetGravityZ` (`Character.CharacterMovement` (`self.OwnerCharacter`))))) (`CharacterMovementComponent.Mass` (`Character.CharacterMovement` (`self.OwnerCharacter`))))))
    (else
      (`self.StopAbility`))))

(event `StopAbility`
  ;[1 1 1] Stop the ability when the time runs up
  (`MRAbilityComponent.StopAbility` (`MRCharacter.AbilityComponent` (`self.OwnerCharacter`)) (struct :`TagName` "Ability.Jump")))

(fn `CanPerformAbility`
  (returns (ReturnValue :type Boolean))
  (return true))