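; Door actor that swings open when its Activable component receives a message matching its OpenMessage.
; OpenDoor gives the RotatingMovement component a constant rotation rate and starts a one-shot timer, with StopOpen zeroing the rate to end the swing.
; The opening angle comes from rate and duration rather than a target rotation, and there is no closing logic or guard against repeated activation.
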(event `self.Activable.OnActivated`
  (params (Message :type "GameplayTag Structure"))
  (if (== Message (`self.OpenMessage`))
    (`self.OpenDoor`)))

(event `OpenDoor`
  (set `RotatingMovementComponent.RotationRate` (struct :`Yaw` 90.0) (`self.RotatingMovement`))
  (`KismetSystemLibrary.K2_SetTimerDelegate` (`|CreateDelegate` :!event `StopOpen`) 1.0))

(event `StopOpen`
  (set `RotatingMovementComponent.RotationRate` (struct) (`self.RotatingMovement`)))

(fn `UserConstructionScript`)