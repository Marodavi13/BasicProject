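; Elevator actor that carries a platform along a spline between its two ends.
; A Pawn entering the trigger box while the elevator is idle fires the Activator component, and the Activable component's activation event starts the movement.
; A timeline drives the movement root along the spline length with sweep, playing or reversing according to the spline key nearest the cube.
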(event `self.Box.OnComponentBeginOverlap`
  (params (OverlappedComponent :type "PrimitiveComponent Object Reference") (OtherActor :type "Actor Object Reference") (OtherComp :type "PrimitiveComponent Object Reference") (OtherBodyIndex :type Integer) (bFromSweep :type Boolean) (SweepResult :type "HitResult Structure (by ref)"))
  (if (and (`KismetMathLibrary.ClassIsChildOf` (`GameplayStatics.GetObjectClass` OtherActor) "/Script/Engine.Pawn") (not (`self.bIsMoving`)))
    (`MRActivatorComponent.ActivateActors` (`self.Activator`))))

(event `self.Activable.OnActivated`
  (params (Message :type "GameplayTag Structure"))
  (set `self.bIsMoving` true)
  (if (< (`KismetMathLibrary.Round` (`SplineComponent.FindInputKeyClosestToWorldLocation` (`self.Spline`) (`SceneComponent.K2_GetComponentLocation` (`self.Cube`)))) 1)
    (bind (_direction _newtrack_0) (`Timeline|ElevatorMovement` :!label _label)
      (:`Update`
        (`SceneComponent.K2_SetRelativeLocation` (`self.ElevatorMovementRoot`) (`SplineComponent.GetLocationAtDistanceAlongSpline` (`self.Spline`) (* _newtrack_0 (`SplineComponent.GetSplineLength` (`self.Spline`))) "Local") true true))
      (:`Finished`
        (set `self.bIsMoving` false)))
    (else
      (goto _label :!via `Reverse`))))

(fn `UserConstructionScript`)